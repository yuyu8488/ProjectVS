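; BP_MonsterVS is a monster character that knocks the player away on contact.
; Capsule overlap with BP_PlayerCharacter launches the player along the monster-to-player direction at fixed speed, overriding existing velocity.
; A CanAttack flag gates a debug hit print but not the launch, and is cleared once the print fires.
; ResetAttackCooldown restores the flag, though nothing in this file calls it.
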(event `self.CapsuleComponent.OnComponentBeginOverlap`
  (params (OverlappedComponent :type "PrimitiveComponent Object Reference") (OtherActor :type "Actor Object Reference") (OtherComp :type "PrimitiveComponent Object Reference") (OtherBodyIndex :type Integer) (bFromSweep :type Boolean) (SweepResult :type "HitResult Structure (by ref)"))
  (bind _asbp_player_character (cast `/Game/Blueprints/Character/BP_PlayerCharacter` OtherActor))
  (`self.LaunchCharacter` _asbp_player_character (* (`KismetMathLibrary.GetForwardVector` (`KismetMathLibrary.FindLookAtRotation` (`self.K2_GetActorLocation`) (`self.K2_GetActorLocation` _asbp_player_character))) 500.0) true true)
  ; Comment
  (if (`self.CanAttack`)
    (set `self.CanAttack` false)
    (`KismetSystemLibrary.PrintString` (`KismetStringLibrary.Concat_StrStr` (`KismetSystemLibrary.GetClassDisplayName` (`GameplayStatics.GetObjectClass` self)) "  Hit ::" (`KismetSystemLibrary.GetClassDisplayName` (`GameplayStatics.GetObjectClass` _asbp_player_character))))))

(fn `ResetAttackCooldown`
  (set `self.CanAttack` true))

(fn `UserConstructionScript`
  (`parent.UserConstructionScript`))