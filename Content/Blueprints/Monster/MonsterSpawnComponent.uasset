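; Actor component that spawns random monsters in a ring around its owner on a half-second looping timer until a spawn count cap is reached.
; Each spawn picks a point on the circle's edge at the set radius, faces the owner and runs the BT_Monster behavior tree.
; Monster classes come from random DT_Monster rows, with row names cached on first use.
; The spawn count only increases within this component.
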(event `self.ReceiveBeginPlay`
  (`KismetSystemLibrary.K2_SetTimer` null "SpawnMonster" 0.5 true))

(fn `GetRandomLocationInCircle`
  (returns (ReturnValue :type "Vector Structure"))
  (locals (`Random Value` :type "Float (double-precision)" :default 0.0))
  (bind _radius (`self.Radius`))
  (bind _output_get (set `local.Random Value` (`KismetMathLibrary.RandomFloatInRange` 0.0 360.0)))
  (bind _returnvalue (`KismetMathLibrary.DegreesToRadians` _output_get))
  (return (+ (`Actor.K2_GetActorLocation` (`self.GetOwner`)) (`KismetMathLibrary.MakeVector` (* (`KismetMathLibrary.Cos` _returnvalue) _radius) (* (`KismetMathLibrary.Sin` _returnvalue) _radius)))))

(fn `GetRandomMonsterClass`
  (returns (NewParam :type "/Game/Blueprints/Character/Monster/BP_MonsterVS Class Reference"))
  (if (`KismetArrayLibrary.Array_IsEmpty` (`self.MonsterClasses`))
    (bind _outrownames (`DataTableFunctionLibrary.GetDataTableRowNames` "/Game/Blueprints/Monster/DT_Monster.DT_Monster"))
    (set `self.MonsterClasses` _outrownames))
  (bind _returnvalue (`|GetDataTableRow` "/Game/Blueprints/Monster/DT_Monster.DT_Monster" (`KismetArrayLibrary.Array_Random` (`self.MonsterClasses`)))
    (:`then`
      (return (`.MonsterClass_5_D3C3616A4E12DD595B8107804B9FCEA3` (break `/Game/Blueprints/Monster/S_Monster` _returnvalue))))))

(fn `SpawnMonster`
  (locals (RandomLocation :type "Vector Structure" :default (0.0 0.0 0.0)))
  (if (< (`self.SpawnedMonsterCount`) (`self.MaxSpawnCount`))
    (bind _output_get (set `local.RandomLocation` (`self.GetRandomLocationInCircle`)))
    (`AIBlueprintHelperLibrary.SpawnAIFromClass` (`self.GetRandomMonsterClass`) "/Game/Blueprints/AI/BT_Monster.BT_Monster" _output_get (`KismetMathLibrary.FindLookAtRotation` (`local.RandomLocation`) (`Actor.K2_GetActorLocation` (`self.GetOwner`))) true null)
    (bind _result (`/Engine/EditorBlueprintResources/StandardMacros.IncrementInt` (`self.SpawnedMonsterCount`))
      (:`  `
        (set `self.SpawnedMonsterCount` _result)))))