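; Fireball skill projectile that flies forward and explodes on the first overlap, with no damage logic in this Blueprint.
; Tick moves it a fixed, unswept step along its forward vector, so speed depends on frame rate.
; Tick also resets the five-second lifespan every frame, so that timer never expires while ticking.
; Sphere overlap spawns an enlarged explosion at the SweepResult actor's location, then destroys the projectile.
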(event `self.ReceiveTick`
  (params (DeltaSeconds :type "Float (single-precision)"))
  (`self.SetLifeSpan` 5.0)
  (`self.K2_AddActorWorldOffset` (* (`self.GetActorForwardVector`) 10.0)))

(event `self.Sphere.OnComponentBeginOverlap`
  (params (OverlappedComponent :type "PrimitiveComponent Object Reference") (OtherActor :type "Actor Object Reference") (OtherComp :type "PrimitiveComponent Object Reference") (OtherBodyIndex :type Integer) (bFromSweep :type Boolean) (SweepResult :type "HitResult Structure (by ref)"))
  (`GameplayStatics.SpawnEmitterAtLocation` "/Game/StarterContent/Particles/P_Explosion.P_Explosion" (`self.K2_GetActorLocation` (`.HitActor` (`GameplayStatics.BreakHitResult` SweepResult))) (struct) (2.0 2.0 2.0))
  (`self.K2_DestroyActor`))

(fn `UserConstructionScript`
  (`parent.UserConstructionScript`))