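; Skill component that holds its owner's skill slots and fires each skill automatically whenever its cooldown elapses.
; AddSkill looks up a DT_Skill row by name and stores it as a slot with a timer.
; Tick advances every timer, then resets finished ones and spawns that skill's actor class ahead of the owner, facing along the first player's camera rotation.
; The spawn step is marked as test code.
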(event `self.ReceiveBeginPlay`)

(event `self.ReceiveTick`
  (params (DeltaSeconds :type "Float (single-precision)"))
  (`self.UpdateCooldown`)
  (`self.ExecuteSkills`))

(fn `Add Skill`
  (params (`Skill Name` :type Name))
  (bind _returnvalue (`|GetDataTableRow` "/Game/Blueprints/Skill/DT_Skill.DT_Skill" `Skill Name`)
    (:`then`
      (`KismetArrayLibrary.Array_AddUnique` (`self.SkillSlot`) (make `/Game/Blueprints/Skill/S_SkillSlot` `Skill Name` 0.0 _returnvalue)))))

(fn `ExecuteSkills`
  (bind _returnvalue (`self.GetOwner`))
  (bind _skillslot (`self.SkillSlot`))
  (if (`KismetArrayLibrary.Array_IsNotEmpty` _skillslot)
    (for (_array_element _array_index) _skillslot
      (bind (_skillrowname _currentcooltime _data) (break `/Game/Blueprints/Skill/S_SkillSlot` _array_element))
      ; Cool Down Check
      (if (>= _currentcooltime (`.CoolTime_7_5CECE98B4B99FB574AAB5593DDBD2C34` (break `/Game/Blueprints/Skill/S_SkillData` _data)))
        (bind (_skillrowname_2 _currentcooltime_2 _data_2) (break `/Game/Blueprints/Skill/S_SkillSlot` (`|GetArrayItem` _skillslot _array_index)))
        (`KismetArrayLibrary.Array_Set` (`self.SkillSlot`) _array_index (make `/Game/Blueprints/Skill/S_SkillSlot` _skillrowname_2 0.0 _data_2))
        ; Test
        (`|SpawnActorFromClass` (`.Class_11_32A7B4584F44FF07586E24AB03CA8AE2` (break `/Game/Blueprints/Skill/S_SkillData` (`.Data_9_9D37D78846CDBB7D0EA89DA68F6D12F0` (break `/Game/Blueprints/Skill/S_SkillSlot` _array_element)))) (`KismetMathLibrary.MakeTransform` (+ (`Actor.K2_GetActorLocation` _returnvalue) (* (`Actor.GetActorForwardVector` _returnvalue) 300.0)) (`PlayerCameraManager.GetCameraRotation` (`PlayerController.PlayerCameraManager` (`GameplayStatics.GetPlayerController` 0)))) "AlwaysSpawn" "MultiplyWithRoot" null null)))))

(fn `UpdateCooldown`
  (bind _skillslot (`self.SkillSlot`))
  (for (_array_element _array_index) _skillslot
    (bind _structout (setmembers `/Game/Blueprints/Skill/S_SkillSlot` :`StructRef` _array_element :`CurrentCoolTime` (+ (`.CurrentCoolTime_6_CF46673E442653AC31E5328B6EEC6F27` (break `/Game/Blueprints/Skill/S_SkillSlot` (`|GetArrayItem` _skillslot _array_index))) (`GameplayStatics.GetWorldDeltaSeconds`))))
    (`KismetArrayLibrary.Array_Set` (`self.SkillSlot`) _array_index _structout)))