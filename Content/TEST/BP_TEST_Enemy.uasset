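; Test enemy character that places itself on world geometry at spawn, then chases the player.
; BeginPlay runs a vertical WorldStatic trace, and a timeline animates its height from the hit point by scaled capsule half-height.
; When the timeline finishes, Tick feeds the direction toward the first BP_PlayerCharacterVS straight into CharacterMovement, without AI navigation.
; Unconnected experiments remain for an alternative spawn trace, slope push-up and AIMoveTo.
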(event `self.ReceiveBeginPlay`
  ; Enemy Spawn
  ;; Comment
  (bind _outhit (`KismetSystemLibrary.LineTraceSingleForObjects` :`Start` (+ (`self.K2_GetActorLocation`) (* (`self.GetActorUpVector`) -1000.0)) :`End` (+ (`self.K2_GetActorLocation`) (* (`self.GetActorUpVector`) 2000.0)) :`ObjectTypes` (`|MakeArray` "ObjectTypeQuery1" :!type "EObjectTypeQuery Enum") :`DrawDebugType` "ForDuration" :`DrawTime` 1.0))
  (bind (_direction _newtrack_0) (`Timeline|Timeline`)
    (:`Update`
      (`self.K2_SetActorLocation` (+ (`.Location` (`GameplayStatics.BreakHitResult` _outhit)) (* (`self.GetActorUpVector`) (* (`CapsuleComponent.CapsuleHalfHeight` (`self.CapsuleComponent`)) _newtrack_0)))))
    (:`Finished`
      ;; AI Move (자동이동)
      (set `self.bSpawnCompleted` true))))

(event `self.ReceiveTick`
  (params (DeltaSeconds :type "Float (single-precision)"))
  (`|ExecutionSequence`
    (:`then_0`
      ; 임시 이동 테스트 (Add Input Vector) 강제 이동
      (if (`self.bSpawnCompleted`)
        (bind _outactors (`GameplayStatics.GetAllActorsOfClass` "/Game/Blueprints/Character/BP_PlayerCharacterVS.BP_PlayerCharacterVS_C"))
        (`PawnMovementComponent.AddInputVector` (`self.CharacterMovement`) (- (`self.K2_GetActorLocation` (`|GetArrayItem` _outactors)) (`self.K2_GetActorLocation`)) false)))))

(fn `UserConstructionScript`)